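; BP_PlayerCharacter is the player character, handling movement, camera look and a basic attack.
; Axis inputs move it along the control rotation's forward and right vectors and drive controller yaw and pitch.
; The Attack input fires a short visibility line trace along the actor's forward vector and applies fixed damage to any hit actor.
; TakeDamageCustom and GainXP simply adjust Health and XP, and neither is called within this Blueprint.
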(event `InputAxis|MoveForward`
  (params (AxisValue :type "Float (single-precision)"))
  (`self.AddMovementInput` (`KismetMathLibrary.GetForwardVector` (`Controller.GetControlRotation` (`self.GetController`))) AxisValue))

(event `InputAxis|MoveRight`
  (params (AxisValue :type "Float (single-precision)"))
  (`self.AddMovementInput` (`KismetMathLibrary.GetRightVector` (`Controller.GetControlRotation` (`self.GetController`))) AxisValue))

(event `InputAxis|Turn`
  (params (AxisValue :type "Float (single-precision)"))
  (`self.AddControllerYawInput` AxisValue))

(event `InputAxis|LookUp`
  (params (AxisValue :type "Float (single-precision)"))
  (`self.AddControllerPitchInput` AxisValue))

(event `InputAction|Attack`
  (params (Key :type "Key Structure"))
  (bind _returnvalue (`self.K2_GetActorLocation`))
  (:`Pressed`
    (bind _outhit (`KismetSystemLibrary.LineTraceSingle` _returnvalue (+ _returnvalue (* (`self.GetActorForwardVector`) (300.0 300.0 300.0))) "TraceTypeQuery1"))
    (bind (_bblockinghit _binitialoverlap _time _distance _location _impactpoint _normal _impactnormal _physmat _hitactor) (`GameplayStatics.BreakHitResult` _outhit))
    (if (`KismetSystemLibrary.IsValid` _hitactor)
      (`self.Attack` _hitactor 25.0))))

(fn `Attack`
  (params (Target :type "Actor Object Reference") (DamageAmount :type "Float (double-precision)"))
  (`GameplayStatics.ApplyDamage` Target DamageAmount))

(fn `GainXP`
  (params (Amount :type Integer))
  (set `self.XP` (+ (`self.XP`) Amount)))

(fn `TakeDamageCustom`
  (params (Amount :type "Float (double-precision)"))
  (set `self.Health` (- (`self.Health`) Amount)))

(fn `UserConstructionScript`)